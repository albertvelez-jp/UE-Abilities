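; AC_ObjectPool is an actor component that pre-spawns and recycles actors of a configurable class.
; On BeginPlay it fills ObjectPool with spawned actors, each marked not in use.
; SpawnFromPool linearly searches for the first free actor, moves it to the given transform and returns it.
; SpawnFromPool sets InUse to false rather than true, so nothing here marks a handed-out actor as taken.
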(event `self.ReceiveBeginPlay`
  (`self.InitializePool`))

(event `InitializePool`
  (for _ (range (+ (`self.PoolSize`) 1))
    (bind _returnvalue (`|SpawnActorFromClass` (`self.PooledActorClass`) (struct) "Undefined" "MultiplyWithRoot" null null))
    (`KismetArrayLibrary.Array_AddUnique` (`self.ObjectPool`) _returnvalue)
    (`/Game/ObjectPool/BP_PooledActor.Setinuse` _returnvalue false)))

(fn `FindFirstAvailableActor`
  (returns (PooledActor :type "/Game/ObjectPool/BP_PooledActor Object Reference"))
  (for _array_element (`self.ObjectPool`)
    (if (not (`/Game/ObjectPool/BP_PooledActor.InUse` _array_element))
      (return _array_element))))

(fn `SpawnFromPool`
  (params (SpawnTransform :type "Transform Structure"))
  (returns (PooledActor :type "/Game/ObjectPool/BP_PooledActor Object Reference"))
  (bind _pooledactor (`self.FindFirstAvailableActor`))
  (`/Engine/EditorBlueprintResources/StandardMacros.IsValid` _pooledactor
    (:`Is Valid`
      (`Actor.K2_SetActorTransform` _pooledactor SpawnTransform false false)
      (`/Game/ObjectPool/BP_PooledActor.Setinuse` _pooledactor false)
      (return _pooledactor))))