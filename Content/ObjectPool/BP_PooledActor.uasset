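; BP_PooledActor is an actor for object pooling that toggles between in-use and idle states, starting idle on BeginPlay.
; Setinuse stores the flag, switches tick on with use and collision the opposite way (off in use, on when idle), and clears the lifetime timer.
; Activation starts a TimeToLive timer whose ReturnToPool event sets the actor idle again, without destroying it or changing its visibility.
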(event `self.ReceiveBeginPlay`
  (`self.Setinuse` false))

(event `Setinuse`
  (params (InUse :type Boolean))
  (set `self.InUse` InUse)
  (`self.SetActorEnableCollision` (not InUse))
  (`self.SetActorTickEnabled` InUse)
  (`KismetSystemLibrary.K2_ClearAndInvalidateTimerHandle` (`self.TimeToLiveTimer`))
  (if InUse
    (bind _returnvalue (`KismetSystemLibrary.K2_SetTimerDelegate` (delegate `ReturnToPool`) (`self.TimeToLive`)))
    (set `self.TimeToLiveTimer` _returnvalue)))

(event `ReturnToPool`
  (`self.Setinuse` false))

(fn `UserConstructionScript`)